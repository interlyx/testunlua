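; Player controller Blueprint bound to a script module by name, holding test functions for passing arrays.
; GetModuleName returns the module path Player.BP_PlayerController_C, in the style of UnLua bindings.
; TestArrayString and TestArrayInt print each element of the array they receive.
; BPTestFunc feeds the Bpintarray variable into TestArrayInt, while the construction script is empty.
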(event `TestArrayString`
  (params (NewParam :type "Array of String (by ref)"))
  (for _array_element NewParam
    (`KismetSystemLibrary.PrintString` _array_element)))

(event `TestArrayInt`
  (params (NewParam :type "Array of Integer (by ref)"))
  (for _array_element NewParam
    (`KismetSystemLibrary.PrintString` (`KismetStringLibrary.Conv_IntToString` _array_element))))

(fn `BPTestFunc`
  (`self.TestArrayInt` (`self.bpintarray`)))

(fn `GetModuleName`
  (returns (ReturnValue :type String))
  (return "Player.BP_PlayerController_C"))

(fn `UserConstructionScript`)